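; BP_PaperNote is a collectible note that the first-person character picks up by pressing Interact while nearby.
; Box overlap with the character enables input and opens a Gate, and leaving disables input and closes it.
; Interacting through the open Gate marks the note's Number as collected in the character's NotesCollected array, plays a sound at its location and destroys the actor.
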(event OnComponentBeginOverlap(Box)
  (params (OverlappedComponent :type Primitive%20Component%20Object%20Reference) (OtherActor :type Actor%20Object%20Reference) (OtherComp :type Primitive%20Component%20Object%20Reference) (OtherBodyIndex :type Integer) (bFromSweep :type Boolean) (SweepResult :type Hit%20Result%20Structure%20%28by%20ref%29))
  (bind _number (Variables|Default|GetNumber))
  (bind _asbp_first_person_character (Utilities|Casting|CastToBP_FirstPersonCharacter OtherActor))
  (Input|EnableInput (Game|GetPlayerController 0))
  (Utilities|FlowControl|Gate true) ; enters at Open
)

(event OnComponentEndOverlap(Box)
  (params (OverlappedComponent :type Primitive%20Component%20Object%20Reference) (OtherActor :type Actor%20Object%20Reference) (OtherComp :type Primitive%20Component%20Object%20Reference) (OtherBodyIndex :type Integer))
  (bind _number (Variables|Default|GetNumber))
  (Utilities|Casting|CastToBP_FirstPersonCharacter OtherActor)
  (Input|DisableInput (Game|GetPlayerController 0))
  (Utilities|FlowControl|Gate true) ; enters at Close
)

(event Input|ActionEvents|InputActionInteract
  (params (Key :type Key%20Structure :default "None"))
  (bind _number (Variables|Default|GetNumber))
  (:Pressed
    (Utilities|FlowControl|Gate true
      (:Exit
        (Utilities|Array|SetArrayElem (Variables|/Game/FirstPerson/Blueprints/BP_FirstPersonCharacter.BP_FirstPersonCharacter_C|GetNotesCollected (stale OnComponentBeginOverlap(Box) _asbp_first_person_character)) (Utilities|Array|FindItem (Variables|/Game/FirstPerson/Blueprints/BP_FirstPersonCharacter.BP_FirstPersonCharacter_C|GetNotesCollected (stale OnComponentBeginOverlap(Box) _asbp_first_person_character)) (Utilities|Struct|MakeSTRUCT_Note _number false)) (Utilities|Struct|MakeSTRUCT_Note _number true))
        (Audio|PlaySoundatLocation 0 (Transformation|GetActorLocation) "0, 0, 0" 1.0 1.0 0.0 0 0 0 0)
        (Actor|DestroyActor)))))

(fn ConstructionScript)