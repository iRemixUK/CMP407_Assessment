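; BP_SlidingDoor is a door that endlessly opens and closes on its own from BeginPlay, with no trigger or player interaction.
; OpenDoor plays the SlidingDoor timeline to lerp the Wall component's relative location downward on Z, then calls CloseDoor when finished.
; CloseDoor uses a second timeline, Timeline_0, to lerp the Wall back to its origin, then calls OpenDoor to repeat the cycle.
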(event Custom|OpenDoor
  (bind _open (Timeline|SlidingDoor PlayFromStart)
    (:Update
      (Transformation|SetRelativeLocation (Variables|Default|GetWall) (Math|Vector|Lerp(Vector) "0, 0, 0" "0, 0,-345.000000" _open) false false))
    (:Finished
      (CallFunction|CloseDoor))))

(event Custom|Close%20door
  (bind _open (Timeline|Timeline_0 PlayFromStart)
    (:Update
      (Transformation|SetRelativeLocation (Variables|Default|GetWall) (Math|Vector|Lerp(Vector) "0, 0,-345.000000" "0, 0,0.000000" _open) false false))
    (:Finished
      (CallFunction|OpenDoor))))

(event EventBeginPlay
  (CallFunction|OpenDoor))

(event Collision|EventActorBeginOverlap
  (params (OtherActor :type Actor%20Object%20Reference)))

(event EventTick
  (params (DeltaSeconds :type Float%20%28single-precision%29)))

(fn ConstructionScript)